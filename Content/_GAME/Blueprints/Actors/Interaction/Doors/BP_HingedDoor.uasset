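; BP_HingedDoor is an interactable hinged door that can be locked or gated behind a player attribute check.
; Until any required check passes, it stays locked and routes look-at and interaction through ACStatInteraction; passing it unlocks the door.
; Otherwise it uses ACSimpleInteraction and parent interaction logic.
; Lock events update the red/green indicator material, prompt widget and mesh highlight.
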(event EventInteract
  (if (State|IsStatCheckHandled)
    (|CallParentFunction)
    (elif (Math|Boolean|ANDBoolean (Variables|Default|GetAllowInteraction) (Variables|Default|GetisInteractable) (Default|HasEnoughAttributeValue (Variables|Default|GetAC_StatInteraction)))
      (State|CompleteStatCheck)
      (|CallParentFunction))))

(event EventOnDoorUnlocked
  (if (State|IsStatCheckHandled)
    (Rendering|Material|SetMaterial (Variables|Default|GetStaticMesh) (Variables|Properties|GetLockIndicatorMaterialIndex) "/Game/Placeholder/Indicator_Green.Indicator_Green")
    (Default|ConfigureWidget (Variables|Default|GetAC_SimpleInteraction) (Variables|Default|GetActionText) (Variables|Properties|GetDisplay%20Input%20Action))
    (if (== (Variables|/Script/Arsenic.ArsenicPlayerCharacter|GetLookAtActor (Variables|Default|GetArsenicPlayerCharacter)) self)
      (Class|ArsenicInteractActorBase|HighlightMesh))))

(event EventLookat
  (|CallParentFunction)
  (if (State|IsStatCheckHandled)
    (Default|SimpleLookat (Variables|Default|GetAC_SimpleInteraction) (Variables|Default|GetAllowInteraction) (Variables|Default|GetActionText))
    (else
      (Default|ComponentLookat (Variables|Default|GetAC_StatInteraction) (Variables|Default|GetAllowInteraction)))))

(event EventStopLookingat
  (if (State|IsStatCheckHandled)
    (Default|RemoveWidget (Variables|Default|GetAC_SimpleInteraction))
    (else
      (Default|RemoveWidget (Variables|Default|GetAC_StatInteraction)))))

(event EventOnActionTextChanged
  (if (Variables|Default|GetDoorLocked)
    (Variables|/Game/_GAME/Blueprints/Components/Interaction/AC_SimpleInteraction.AC_SimpleInteraction_C|SetDisplayInputAction (Variables|Default|GetAC_SimpleInteraction) "")
    (Default|SetActionText (Variables|Default|GetAC_SimpleInteraction) (Variables|Default|GetActionText))
    (else
      (Default|SetActionText (Variables|Default|GetAC_SimpleInteraction) (Variables|Default|GetActionText))
      (Variables|/Game/_GAME/Blueprints/Components/Interaction/AC_SimpleInteraction.AC_SimpleInteraction_C|SetDisplayInputAction (Variables|Default|GetAC_SimpleInteraction) (Variables|Properties|GetDisplay%20Input%20Action)))))

(event EventOnDoorLocked
  (Rendering|Material|SetMaterial (Variables|Default|GetStaticMesh) (Variables|Properties|GetLockIndicatorMaterialIndex) "/Game/Placeholder/Indicator_Red.Indicator_Red")
  (Default|ConfigureWidget (Variables|Default|GetAC_SimpleInteraction) (Variables|Default|GetActionText))
  (if (Variables|Default|GetisHighlighted)
    (Class|ArsenicInteractActorBase|UnHighlightMesh)))

(event EventOnDoorStateLoaded
  (if (State|IsStatCheckHandled)
    (if (Variables|Default|GetDoorLocked)
      (Class|ArsenicDoorBase|LockDoor)
      (else
        (Class|ArsenicDoorBase|UnlockDoor)))
    (else
      (Class|ArsenicDoorBase|LockDoor))))

(fn ConstructionScript)

(fn ConfigureDoor
  (params (Default%20Door%20Speed :type Float%20%28single-precision%29) (Close%20Door%20Automatically :type Boolean) (Slam%20Speed%20Multiplier :type Float%20%28single-precision%29) (Distance%20to%20Close :type Float%20%28single-precision%29))
  (Variables|Default|SetDefaultDoorSpeed Default%20Door%20Speed)
  (Variables|Default|SetCloseDoorAutomatically Close%20Door%20Automatically)
  (Variables|Default|SetSlamSpeedMultiplier Slam%20Speed%20Multiplier)
  (Variables|Default|SetDistanceToClose Distance%20to%20Close))

(fn IsStatCheckHandled
  (return (or (not (Variables|Default|GetRequiresStatCheck)) (Variables|Default|GetStatInteractionSuccessful))))

(fn CompleteStatCheck
  (Default|RemoveWidget (Variables|Default|GetAC_StatInteraction))
  (Variables|Default|SetStatInteractionSuccessful true)
  (Class|ArsenicDoorBase|UnlockDoor))