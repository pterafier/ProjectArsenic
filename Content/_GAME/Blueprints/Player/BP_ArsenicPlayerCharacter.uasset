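; BP_ArsenicPlayerCharacter is the player character Blueprint, whose visible logic consists only of debug key bindings.
; DebugKey1 applies GE_TestEffect to the character through the player state's ArsenicAbilitySystemComponent.
; DebugKey2 and DebugKey3 lock and unlock every ArsenicDoorBase actor found in the level.
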(event Input|KeyboardEvents|DebugKey1
  (params (Key :type Key%20Structure :default "None") (ActionValue :type Input%20Action%20Value%20Structure))
  (:Pressed
    (bind _asarsenic_ability_system_component (Utilities|Casting|CastToArsenicAbilitySystemComponent (Ability|GetAbilitySystemComponent (Variables|Default|GetArsenicPlayerState))))
    (Class|ArsenicAbilitySystemComponent|ApplyEffecttoTarget _asarsenic_ability_system_component self "/Game/_GAME/Blueprints/AbilitySystem/Effects/Testing/GE_TestEffect.GE_TestEffect_C" 1.0)))

(event Input|KeyboardEvents|DebugKey2
  (params (Key :type Key%20Structure :default "None") (ActionValue :type Input%20Action%20Value%20Structure))
  (:Pressed
    (bind _outactors (Actor|GetAllActorsOfClass "/Script/Arsenic.ArsenicDoorBase"))
    (for _array_element _outactors
      (Class|ArsenicDoorBase|LockDoor _array_element))))

(event Input|KeyboardEvents|DebugKey3
  (params (Key :type Key%20Structure :default "None") (ActionValue :type Input%20Action%20Value%20Structure))
  (:Pressed
    (bind _outactors (Actor|GetAllActorsOfClass "/Script/Arsenic.ArsenicDoorBase"))
    (for _array_element _outactors
      (Class|ArsenicDoorBase|UnlockDoor _array_element))))

(fn ConstructionScript)