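; Actor component that shows a simple interaction prompt, with action text and an input action, on the player HUD.
; When interaction is allowed, SimpleLookAt creates a WB_SimpleInteractionPopup and swaps it into the HUD's interact slot, replacing existing children.
; Other functions update the popup's text or input action, or clear the slot.
; SimpleLookAt and RemoveWidget lazily cache the player controller and HUD references via SetReferences.
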(event EventBeginPlay)

(event EventTick
  (params (DeltaSeconds :type Float%20%28single-precision%29)))

(fn CreateSimpleWidget
  (params (ActionText :type Text))
  (bind _returnvalue (UserInterface|CreateWidget "/Game/_GAME/UI/Widgets/HUD/Interaction/WB_SimpleInteractionPopup.WB_SimpleInteractionPopup_C" (Variables|Default|GetBP_ArsenicPlayerController)))
  (bind _output_get (Variables|Default|SetWB_SimpleInteractionPopup _returnvalue))
  (Default|ConfigureWidget _output_get (Utilities|Array|MakeArray (Variables|Default|GetDisplayInputAction)) ActionText)
  (if (Class|PanelWidget|HasAnyChildren (Variables|/Game/_GAME/UI/Widgets/HUD/WB_ArsenicPlayerHUD.WB_ArsenicPlayerHUD_C|GetVB_InteractWidgetSlot (Variables|Default|GetWB_ArsenicPlayerHUD)))
    (Widget|Panel|ClearChildren (Variables|/Game/_GAME/UI/Widgets/HUD/WB_ArsenicPlayerHUD.WB_ArsenicPlayerHUD_C|GetVB_InteractWidgetSlot (Variables|Default|GetWB_ArsenicPlayerHUD))))
  (Class|VerticalBox|AddChildtoVerticalBox (Variables|/Game/_GAME/UI/Widgets/HUD/WB_ArsenicPlayerHUD.WB_ArsenicPlayerHUD_C|GetVB_InteractWidgetSlot (Variables|Default|GetWB_ArsenicPlayerHUD)) (Variables|Default|GetWB_SimpleInteractionPopup)))

(fn SetReferences
  (bind _asbp_arsenic_player_controller (Utilities|Casting|CastToBP_ArsenicPlayerController (Game|GetPlayerController 0)))
  (bind _output_get (Variables|Default|SetBP_ArsenicPlayerController _asbp_arsenic_player_controller))
  (bind _aswb_arsenic_player_hud (Utilities|Casting|CastToWB_ArsenicPlayerHUD (Variables|/Script/Arsenic.PlayerHUD|GetArsenicPlayerHUD (Variables|/Script/Arsenic.ArsenicPlayerController|GetPlayerHUDActor _output_get))))
  (Variables|Default|SetWB_ArsenicPlayerHUD _aswb_arsenic_player_hud))

(fn SetActionText
  (params (ActionText :type Text))
  (bind _wb_simpleinteractionpopup (Variables|Default|GetWB_SimpleInteractionPopup))
  (Utilities|IsValid _wb_simpleinteractionpopup
    (:Is%20Valid
      (Rendering|Components|TextRender|SetText (Variables|/Game/_GAME/UI/Widgets/HUD/Interaction/WB_SimpleInteractionPopup.WB_SimpleInteractionPopup_C|GetActionText _wb_simpleinteractionpopup) ActionText))))

(fn RemoveWidget
  (Utilities|IsValid (Variables|Default|GetWB_ArsenicPlayerHUD)
    (:Is%20Valid
      _)
    (:Is%20Not%20Valid
      (CallFunction|SetReferences)))
  (if (Class|PanelWidget|HasAnyChildren (Variables|/Game/_GAME/UI/Widgets/HUD/WB_ArsenicPlayerHUD.WB_ArsenicPlayerHUD_C|GetVB_InteractWidgetSlot (Variables|Default|GetWB_ArsenicPlayerHUD)))
    (Widget|Panel|ClearChildren (Variables|/Game/_GAME/UI/Widgets/HUD/WB_ArsenicPlayerHUD.WB_ArsenicPlayerHUD_C|GetVB_InteractWidgetSlot (Variables|Default|GetWB_ArsenicPlayerHUD)))))

(fn SimpleLookat
  (params (AllowInteraction :type Boolean) (ActionText :type Text))
  (Utilities|IsValid (Variables|Default|GetBP_ArsenicPlayerController)
    (:Is%20Valid
      _)
    (:Is%20Not%20Valid
      (CallFunction|SetReferences)))
  (if AllowInteraction
    (CallFunction|CreateSimpleWidget ActionText)))

(fn ConfigureWidget
  (params (ActionText :type Text) (InputAction :type Data%20Table%20Row%20Handle%20Structure))
  (bind _wb_simpleinteractionpopup (Variables|Default|GetWB_SimpleInteractionPopup))
  (Utilities|IsValid _wb_simpleinteractionpopup
    (:Is%20Valid
      (Default|ConfigureWidget _wb_simpleinteractionpopup (Utilities|Array|MakeArray InputAction) ActionText))))