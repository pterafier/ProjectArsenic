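; Interaction component that gates an interaction on a player gameplay attribute and shows a stat-check popup when looked at.
; On BeginPlay it caches the player's ability system component from the character or player state, then compares the chosen attribute against a required value.
; Look-at builds a configured popup with current and required amounts in the HUD's interact slot, resolving controller and HUD references lazily; RemoveWidget clears it.
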(event EventBeginPlay
  (bind _output_get (Variables|Default|SetPlayerASC (Ability|GetAbilitySystemComponent (Game|GetPlayerCharacter 0))))
  (Utilities|IsValid _output_get
    (:Is%20Not%20Valid
      (Variables|Default|SetPlayerASC (Ability|GetAbilitySystemComponent (Game|GetPlayerState 0))))))

(fn HasEnoughAttributeValue
  (Utilities|IsValid (Variables|Default|GetPlayerASC)
    (:Is%20Valid
      (return (>= (.ReturnValue (Class|AbilitySystemComponent|GetGameplayAttributeValue (Variables|Default|GetPlayerASC) (Variables|Default|GetAttributeToCheck))) (Variables|Default|GetRequiredAttributeValue))))))

(fn SetReferences
  (bind _asbp_arsenic_player_controller (Utilities|Casting|CastToBP_ArsenicPlayerController (Game|GetPlayerController 0)))
  (bind _output_get (Variables|Default|SetBP_ArsenicPlayerController _asbp_arsenic_player_controller))
  (bind _aswb_arsenic_player_hud (Utilities|Casting|CastToWB_ArsenicPlayerHUD (Variables|/Script/Arsenic.PlayerHUD|GetArsenicPlayerHUD (Variables|/Script/Arsenic.ArsenicPlayerController|GetPlayerHUDActor _output_get))))
  (Variables|Default|SetWB_ArsenicPlayerHUD _aswb_arsenic_player_hud))

(fn CreateStatCheckWidget
  (bind _returnvalue (UserInterface|CreateWidget "/Game/_GAME/UI/Widgets/HUD/Interaction/WB_StatInteractionPopup.WB_StatInteractionPopup_C" (Variables|Default|GetBP_ArsenicPlayerController)))
  (bind _output_get (Variables|Default|SetWB_StatInteractionPopup _returnvalue))
  (Default|ConfigureWidget _output_get (Utilities|Array|MakeArray (Variables|Default|GetDisplayInputAction)) (Variables|Default|GetAction%20Icon) (Variables|Default|GetActionText) (Variables|Default|GetStat%20Icon) (Math|Float|Truncate (.ReturnValue (Class|AbilitySystemComponent|GetGameplayAttributeValue (Variables|Default|GetPlayerASC) (Variables|Default|GetAttributeToCheck)))) (Math|Float|Truncate (Variables|Default|GetRequiredAttributeValue)))
  (if (Class|PanelWidget|HasAnyChildren (Variables|/Game/_GAME/UI/Widgets/HUD/WB_ArsenicPlayerHUD.WB_ArsenicPlayerHUD_C|GetVB_InteractWidgetSlot (Variables|Default|GetWB_ArsenicPlayerHUD)))
    (Widget|Panel|ClearChildren (Variables|/Game/_GAME/UI/Widgets/HUD/WB_ArsenicPlayerHUD.WB_ArsenicPlayerHUD_C|GetVB_InteractWidgetSlot (Variables|Default|GetWB_ArsenicPlayerHUD))))
  (Class|VerticalBox|AddChildtoVerticalBox (Variables|/Game/_GAME/UI/Widgets/HUD/WB_ArsenicPlayerHUD.WB_ArsenicPlayerHUD_C|GetVB_InteractWidgetSlot (Variables|Default|GetWB_ArsenicPlayerHUD)) (Variables|Default|GetWB_StatInteractionPopup)))

(fn RemoveWidget
  (Utilities|IsValid (Variables|Default|GetWB_ArsenicPlayerHUD)
    (:Is%20Valid
      _)
    (:Is%20Not%20Valid
      (CallFunction|SetReferences)))
  (if (Class|PanelWidget|HasAnyChildren (Variables|/Game/_GAME/UI/Widgets/HUD/WB_ArsenicPlayerHUD.WB_ArsenicPlayerHUD_C|GetVB_InteractWidgetSlot (Variables|Default|GetWB_ArsenicPlayerHUD)))
    (Widget|Panel|ClearChildren (Variables|/Game/_GAME/UI/Widgets/HUD/WB_ArsenicPlayerHUD.WB_ArsenicPlayerHUD_C|GetVB_InteractWidgetSlot (Variables|Default|GetWB_ArsenicPlayerHUD)))))

(fn ComponentLookat
  (params (AllowInteraction :type Boolean))
  (Utilities|IsValid (Variables|Default|GetBP_ArsenicPlayerController)
    (:Is%20Valid
      _)
    (:Is%20Not%20Valid
      (CallFunction|SetReferences)))
  (if AllowInteraction
    (CallFunction|CreateStatCheckWidget)))

(fn ConfigureStatWidget
  (params (Action%20Icon :type Texture%202D%20Object%20Reference) (ActionText :type Text) (Stat%20Icon :type Texture%202D%20Object%20Reference) (DisplayInputAction :type Data%20Table%20Row%20Handle%20Structure))
  (Variables|Default|SetAction%20Icon Action%20Icon)
  (Variables|Default|SetActionText ActionText)
  (Variables|Default|SetStat%20Icon Stat%20Icon)
  (Variables|Default|SetDisplayInputAction DisplayInputAction))